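; Explosive pickup for a ball game that awards no points and blasts the player's ball on pickup.
; BeginPlay disables the number text widget, sets explosion sound and particles for the parent pickup logic, and plays a spark sound at its location.
; On pickup by a BallPawn, it applies a velocity-change radial impulse to the ball mesh from an offset origin, then calls the parent handler.
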(event `self.ReceiveBeginPlay`
  (set `self.UseNumberTextWidget` false)
  (set `self.points` 0)
  (set `self.pickupSound` "/Game/RetroSoundEffects1/Wavs/Explosion_1.Explosion_1")
  (set `self.pickupParticles` "/Game/StarterContent/Particles/P_Explosion.P_Explosion")
  (`GameplayStatics.PlaySoundAtLocation` "/Game/StarterContent/Audio/Fire_Sparks01_CuePinkBall.Fire_Sparks01_CuePinkBall" (`self.K2_GetActorLocation`) (struct) 1.0 1.0 0.0 null null null)
  (`parent.ReceiveBeginPlay`))

(event `self.OnPickup`
  (params (`Other Actor Object` :type "Object Object Reference"))
  (bind _asball_pawn (cast `/Game/Blueprints/BallPawn` `Other Actor Object`))
  (`PrimitiveComponent.AddRadialImpulse` (`/Game/Blueprints/BallPawn.BallMesh` _asball_pawn) (+ (`self.K2_GetActorLocation`) (-100.0 0.0 -50.0)) 200.0 2000.0 "RIF_Constant" true)
  (`parent.OnPickup` `Other Actor Object`))

(fn `UserConstructionScript`
  (`parent.UserConstructionScript`))