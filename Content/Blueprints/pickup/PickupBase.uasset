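; Base pickup actor that awards its Points to a BallPawn that overlaps its sphere.
; OnPickup increments and prints the score, plays a sound and spawns particles.
; With UseNumberTextWidget it swaps the mesh for an animated PickupText widget showing the points, otherwise it destroys itself immediately.
; The overlap event also destroys the actor after a short delay, even when the overlapping actor is not a BallPawn.
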(event `self.ReceiveBeginPlay`
  (bind _pickupwidget (`self.PickupWidget`))
  (`SceneComponent.SetVisibility` _pickupwidget false false)
  (bind _aspickup_text (cast `/Game/Blueprints/pickup/PickupText` (`WidgetComponent.GetUserWidgetObject` _pickupwidget)))
  (set `/Game/Blueprints/pickup/PickupText.ScoreValue` (`self.points`) _aspickup_text))

(event `self.Sphere.OnComponentBeginOverlap`
  (params (OverlappedComponent :type "PrimitiveComponent Object Reference") (OtherActor :type "Actor Object Reference") (OtherComp :type "PrimitiveComponent Object Reference") (OtherBodyIndex :type Integer) (bFromSweep :type Boolean) (SweepResult :type "HitResult Structure (by ref)"))
  (`self.OnPickup` OtherActor)
  (`KismetSystemLibrary.Delay` 1.0)
  (`self.K2_DestroyActor`))

(fn `OnPickup`
  (params (`Other Actor Object` :type "Object Object Reference"))
  ;[1 1 1] Increment Score
  (bind _asball_pawn (cast `/Game/Blueprints/BallPawn` `Other Actor Object`))
  (`/Game/Blueprints/BallPawn.IncrementScore` _asball_pawn (`self.points`))
  (`|ExecutionSequence`
    (:`then_0`
      ;[1 1 1] Play Sound
      (`GameplayStatics.PlaySound2D` (`self.pickupSound`) 1.0 1.0 0.0 null null)
      ;[1 1 1] Emitter
      (`GameplayStatics.SpawnEmitterAtLocation` (`self.pickupParticles`) (`self.K2_GetActorLocation`))
      (if (`self.UseNumberTextWidget`)
        ;[1 1 1] Visibilty (Widget and Mesh)
        (`SceneComponent.SetVisibility` (`self.PickupWidget`) true false)
        (`SceneComponent.SetVisibility` (`self.StaticMesh`) false false)
        ;[1 1 1] More
        (bind _aspickup_text (cast `/Game/Blueprints/pickup/PickupText` (`WidgetComponent.GetUserWidgetObject` (`self.PickupWidget`))))
        (`UserWidget.PlayAnimation` _aspickup_text (`/Game/Blueprints/pickup/PickupText.PickupTextAnimation` _aspickup_text) 0.0 1 "Forward" 1.0 false)
        (else
          (`self.K2_DestroyActor`))))
    (:`then_1`
      (`KismetSystemLibrary.PrintString` (`KismetStringLibrary.Concat_StrStr` "The Score for Coin Pickup is = " (`KismetStringLibrary.Conv_IntToString` (`/Game/Blueprints/BallPawn.Score` _asball_pawn))) true true (struct :`G` 0.66 :`B` 1.0 :`A` 1.0) 10.0))))

(fn `UserConstructionScript`)